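; BP_ServerSubsystem handles network server events and relays new client connections to all players.
; On connect, it wraps the client's ID and status in a ServerClientConnecting struct, then broadcasts it reliably as an instanced struct packet.
; Start, stop and packet-receive events only print debug strings, with received packets logging client ID and length.
; The disconnect handler is empty, and a leftover loop is never executed.
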(event `self.BP_OnServerStartEvent`
  (`KismetSystemLibrary.PrintString` null "ServerStart"))

(event `self.BP_OnServerStopEvent`
  (`KismetSystemLibrary.PrintString` null "ServerStop"))

(event `self.BP_OnClientConnectEvent`
  (params (ClientID :type Integer) (Status :type "EExoPlayerStatus Enum" :default "Connecting"))
  (bind _returnvalue (`StructUtilsFunctionLibrary.MakeInstancedStruct` (make `ServerClientConnectingStruct` ClientID Status)))
  (`self.SendToAllPlayers` _returnvalue))

(event `self.BP_OnClientDisconnectEvent`
  (params (ClientID :type Integer)))

(event `self.BP_OnReceivePacketEvent`
  (params (ClientID :type Integer) (packetLength :type Integer))
  (`KismetSystemLibrary.PrintString` null (`KismetStringLibrary.Concat_StrStr` (`KismetStringLibrary.Conv_IntToString` ClientID) " " (`KismetStringLibrary.Conv_IntToString` packetLength))))